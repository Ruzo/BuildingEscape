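; Openable door actor that swings open and shut when it receives open and close requests through OpenDoor events.
; The DoorSwing timeline plays forward or in reverse, adding a yaw offset to the rotation cached at BeginPlay.
; The timeline's Open Sound event track checks direction, playing a lock sound while opening, or a slam sound with a spark emitter while closing.
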(event `self.ReceiveBeginPlay`
  (bind _output_get (set `self.Initial_Rotation` (`self.K2_GetActorRotation`))))

(event `self.OpenDoor.OnOpenRequest`
  (bind _returnvalue (`self.K2_GetActorLocation`))
  (bind (_direction _rotation) (`Timeline|Door Swing` :!label _label)
    (:`Update`
      (`self.SetActorRotation` (`KismetMathLibrary.ComposeRotators` (stale `self.ReceiveBeginPlay` _output_get) (`KismetMathLibrary.MakeRotator` 0.0 0.0 _rotation))))
    (:`Open Sound`
      (switch `ETimelineDirection` _direction
        (:`Forward`
          (`GameplayStatics.PlaySoundAtLocation` "/Game/door-lock.door-lock" _returnvalue))
        (:`Backward`
          (`|ExecutionSequence`
            (:`then_0`
              (`GameplayStatics.PlaySoundAtLocation` "/Game/Large_Door_Slam.Large_Door_Slam" _returnvalue (struct) 1.0 1.0 0.3))
            (:`then_1`
              (`GameplayStatics.SpawnEmitterAtLocation` "/Game/P_Sparks2.P_Sparks2" _returnvalue (stale `self.ReceiveBeginPlay` _output_get) false))))))))

(event `self.OpenDoor.OnCloseRequest`
  (goto _label :!via `Reverse`))

(fn `UserConstructionScript`)